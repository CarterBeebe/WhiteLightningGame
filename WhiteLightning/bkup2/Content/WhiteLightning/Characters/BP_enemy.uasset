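; BP_enemy is an enemy actor with a paper sprite that fires bullets and can be destroyed by damage.
; A looping timer set at BeginPlay calls shoot, which spawns Bullet_Enemy at the ArrowShot component's transform.
; Enemy_Hit briefly swaps to a shot sprite as hit feedback, restores the main sprite, then subtracts damage from EnemyHealth and destroys the actor when health runs out.
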(event Custom|Enemy_Hit
  (params (Damage :type Float%20%28single-precision%29))
  ;[1 1 1] when the enemy is hit with bullet
  (Rendering|Components|Sprite|SetSprite (Variables|Default|GetPaperSprite) "/Game/WhiteLightning/Sprites/MainEnemyShot_Sprite_2.MainEnemyShot_Sprite_2")
  (Utilities|FlowControl|Delay 0.1)
  (Rendering|Components|Sprite|SetSprite (Variables|Default|GetPaperSprite) "/Game/WhiteLightning/Sprites/MainEnemy_Sprite_2.MainEnemy_Sprite_2")
  (bind _output_get (Variables|Default|Setenemy_Health (- (Variables|Default|Getenemy_Health) Damage)))
  (if (<= _output_get 0.0)
    (Actor|DestroyActor)))

(event Custom|shoot
  (Game|SpawnActorfromClass "/Game/WhiteLightning/Levels/Bullet_Enemy.Bullet_Enemy_C" (Transformation|GetWorldTransform (Variables|Default|GetArrowShot)) "Undefined" 0 0))

(event EventBeginPlay
  (Utilities|Time|SetTimerbyFunctionName 0 "shoot" 2.0 true))

(event Collision|EventActorBeginOverlap
  (params (OtherActor :type Actor%20Object%20Reference)))

(event EventTick
  (params (DeltaSeconds :type Float%20%28single-precision%29)))

(fn ConstructionScript)