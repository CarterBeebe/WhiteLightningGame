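; BP_enemy is a 2D Paper sprite enemy that fires bullets and flashes when hit.
; A looping timer started on BeginPlay calls shoot, which spawns Bullet_Enemy at the ArrowShot component's transform.
; The Enemy_Hit event briefly swaps the sprite to a shot variant and then sets the normal one, with no damage or health handling here.
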(event Custom|Enemy_Hit
  (Rendering|Components|Sprite|SetSprite (Variables|Default|GetPaperSprite) "/Game/WhiteLightning/Sprites/MainEnemyShot_Sprite_2.MainEnemyShot_Sprite_2")
  (Utilities|FlowControl|Delay 0.1)
  (Rendering|Components|Sprite|SetSprite (Variables|Default|GetPaperSprite) "/Game/WhiteLightning/Sprites/MainEnemy_Sprite_2.MainEnemy_Sprite_2"))

(event Custom|shoot
  (Game|SpawnActorfromClass "/Game/WhiteLightning/Levels/Bullet_Enemy.Bullet_Enemy_C" (Transformation|GetWorldTransform (Variables|Default|GetArrowShot)) "Undefined" 0 0))

(event EventBeginPlay
  (Utilities|Time|SetTimerbyFunctionName 0 "shoot" 2.0 true))

(event Collision|EventActorBeginOverlap
  (params (OtherActor :type Actor%20Object%20Reference)))

(event EventTick
  (params (DeltaSeconds :type Float%20%28single-precision%29)))

(fn ConstructionScript)