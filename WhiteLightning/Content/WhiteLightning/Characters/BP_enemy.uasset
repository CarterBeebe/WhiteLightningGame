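; BP_enemy is a 2D Paper sprite enemy that fires bullets on a fixed interval.
; A looping timer set on BeginPlay calls shoot, which spawns Bullet_Enemy at the ArrowShot transform.
; Enemy_Hit briefly swaps to a shot sprite as hit feedback, while Impact prints a debug message and destroys the actor.
; The construction script keeps X and Z but resets Y, snapping the enemy onto the 2D gameplay plane.
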(event Custom|Enemy_Hit
  ;[1 1 1] change sprite when hit
  (Rendering|Components|Sprite|SetSprite (Variables|Default|GetPaperSprite) "/Game/WhiteLightning/Sprites/MainEnemyShot_Sprite_2.MainEnemyShot_Sprite_2")
  (Utilities|FlowControl|Delay 0.2)
  (Rendering|Components|Sprite|SetSprite (Variables|Default|GetPaperSprite) "/Game/WhiteLightning/Sprites/MainEnemy_Sprite_2.MainEnemy_Sprite_2"))

(event Custom|shoot
  ;[1 1 1] Spawing bullets
  (Game|SpawnActorfromClass "/Game/WhiteLightning/Levels/Bullet_Enemy.Bullet_Enemy_C" (Transformation|GetWorldTransform (Variables|Default|GetArrowShot)) "Undefined" 0 0))

(event Custom|Impact
  ;[1 1 1] what happens when hit
  (Development|PrintString "HIT")
  (Actor|DestroyActor))

(event EventBeginPlay
  ;[1 1 1] when game starts constructor
  (Utilities|Time|SetTimerbyFunctionName 0 "shoot" 2.0 true))

(event Collision|EventActorBeginOverlap
  (params (OtherActor :type Actor%20Object%20Reference)))

(event EventTick
  (params (DeltaSeconds :type Float%20%28single-precision%29)))

(fn ConstructionScript
  (bind _returnvalue (Transformation|GetActorLocation))
  (Transformation|SetActorLocation (Math|Vector|MakeVector (.x _returnvalue) 0.0 (.z _returnvalue)) false false))